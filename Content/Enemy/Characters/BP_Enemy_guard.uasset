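; Guard enemy character that plays a guard animation, takes damage and dies when its health runs out.
; A widget health bar updates every tick from the health ratio and rotates to face the player camera.
; AnyDamage subtracts health; on death the guard disables capsule collision and movement, notifies the player character through DecreaseEnemyMessage, plays a dying animation and destroys itself after a delay.
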(event Custom|Death
  ;[0.15 0.15 0.15 0.5] Death
  (Collision|SetCollisionEnabled (Variables|Collision|GetCapsuleComponent) "NoCollision")
  (Class|BPIDecreaaseEnemy|DecreaseEnemy(Message) (Game|GetPlayerCharacter 0))
  (Pawn|Components|CharacterMovement|SetMovementMode (Variables|Character|GetCharacterMovement) "MOVE_None" 0)
  (Components|Animation|PlayAnimation (Variables|Character|GetMesh) "/Game/Characters/imported/Doozy/Dying_Backwards.Dying_Backwards" false)
  (Utilities|FlowControl|Delay 3.0)
  (Actor|DestroyActor))

(event Game|Damage|EventAnyDamage
  (params (Damage :type Float%20%28single-precision%29) (DamageType :type Damage%20Type%20Object%20Reference) (InstigatedBy :type Controller%20Object%20Reference) (DamageCauser :type Actor%20Object%20Reference))
  ;[0.15 0.15 0.15 0.5] Taking damage
  (if (> (Variables|Default|GetHealth) 0.0)
    (bind _output_get (Variables|Default|SetHealth (- (Variables|Default|GetHealth) Damage)))
    (if (<= _output_get 0.0)
      (Variables|Default|SetAllive false)
      (CallFunction|Death))))

(event EventBeginPlay
  (Utilities|FlowControl|Sequence
    (:then_0
      ;[0.15 0.15 0.15 0.5] HealtBar
      (bind _aswb_health_bar (Utilities|Casting|CastToWB_HealthBar (UserInterface|GetUserWidgetObject (Variables|Default|GetHealtBar))))
      (Variables|Default|SetAs%20WB%20Health%20Bar _aswb_health_bar))
    (:then_1
      ;[0.15 0.15 0.15 0.5] Moving
      (Components|Animation|PlayAnimation (Variables|Character|GetMesh) "/Game/Characters/imported/guard_better/Guard_Anim.Guard_Anim" (Variables|Default|GetAllive)))))

(event EventTick
  (params (DeltaSeconds :type Float%20%28single-precision%29))
  (bind _healtbar (Variables|Default|GetHealtBar))
  ;[0.15 0.15 0.15 0.5] HealtBar
  (Progress|SetPercent (Variables|/Game/HUD/WB_HealthBar.WB_HealthBar_C|GetHealtBar (Variables|Default|GetAs%20WB%20Health%20Bar)) (/ (Variables|Default|GetHealth) (Variables|Default|GetMaxHealth)))
  (Transformation|SetWorldRotation _healtbar (Math|Rotator|FindLookatRotation (Transformation|GetWorldLocation _healtbar) (Transformation|GetWorldLocation (Variables|/Script/Engine.PlayerCameraManager|GetTransformComponent (Game|GetPlayerCameraManager 0)))) false false))

(fn ConstructionScript)