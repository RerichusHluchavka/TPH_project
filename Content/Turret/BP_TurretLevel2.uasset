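; BP_TurretLevel2 is a level 2 turret that shoots projectiles at guard enemies it sees.
; PawnSensing detects pawns, and any BP_Enemy_guard becomes the current target.
; After a short delay it spawns a BP_ProjectileTurretLevel2 aimed at that target from one of two muzzle scene components chosen at random.
; Firing is driven solely by sight events, with no separate fire timer.
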(event OnSeePawn(PawnSensing)
  (params (Pawn :type Pawn%20Object%20Reference))
  ;[0.15 0.15 0.15 0.5] Shooting
  (bind _asbp_enemy_guard (Utilities|Casting|CastToBP_Enemy_guard Pawn))
  (Variables|Default|SetCurrentTarget _asbp_enemy_guard)
  (Utilities|FlowControl|Delay 1.0)
  (Game|SpawnActorfromClass "/Game/Turret/BP_ProjectileTurretLevel2.BP_ProjectileTurretLevel2_C" (Transformation|GetWorldTransform (Utilities|Select :Index (Math|Random|RandomIntegerinRange 0 1) :Option%200 (Variables|Default|GetScene) :Option%201 (Variables|Default|GetScene1))) "Undefined" "OverrideRootScale" self (Variables|Default|GetCurrentTarget) 0))

(fn ConstructionScript)