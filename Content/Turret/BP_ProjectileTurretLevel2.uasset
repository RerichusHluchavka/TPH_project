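; Homing projectile for the level 2 turret that chases a Target actor and damages what it hits.
; Each tick it re-aims the ProjectileMovement velocity straight at the target at a set Speed and rotates to face that direction.
; It destroys itself when the target becomes invalid, after a short lifetime, or on a Box collision hit, which also applies fixed damage to the hit actor.
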(event OnComponentHit(Box)
  (params (HitComponent :type Primitive%20Component%20Object%20Reference) (OtherActor :type Actor%20Object%20Reference) (OtherComp :type Primitive%20Component%20Object%20Reference) (NormalImpulse :type Vector :default "0, 0, 0") (Hit :type Hit%20Result%20Structure%20%28by%20ref%29))
  (Actor|DestroyActor)
  (Game|Damage|ApplyDamage (.HitActor (Collision|BreakHitResult Hit)) 6e+01 0 0))

(event Custom|Aim%20At%20Target
  (bind _output_get (Variables|/Script/Engine.MovementComponent|SetVelocity (Variables|Components|GetProjectileMovement) (* (Math|Vector|GetUnitDirection(Vector) (Transformation|GetActorLocation) (Transformation|GetActorLocation (Variables|Default|GetTarget))) (Variables|Default|GetSpeed))))
  (Transformation|SetActorRotation (Math|Conversions|RotationFromXVector _output_get)))

(event EventTick
  (params (DeltaSeconds :type Float%20%28single-precision%29))
  (Variables|Default|GetTarget
    (:then
      (CallFunction|AimatTarget))
    (:else
      (Actor|DestroyActor))))

(event EventBeginPlay
  (Utilities|FlowControl|Delay 5.0)
  (Actor|DestroyActor))

(fn ConstructionScript)