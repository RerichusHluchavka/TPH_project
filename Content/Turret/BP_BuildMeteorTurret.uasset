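; BP_BuildMeteorTurret is the placement preview for building a turret, showing whether it can go at its location.
; Each Tick a box trace flags obstructions and swaps Base and Middle between build and can't-build materials, also factoring in player Money.
; BuildTurret charges the player and spawns the character's Turret class at its TurretBuild transform.
; The preview's money threshold (10) is lower than the build cost (15).
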(event EventTick
  (params (DeltaSeconds :type Float%20%28single-precision%29))
  (bind _returnvalue (Transformation|GetActorLocation))
  (bind _returnvalue_2 (Class|KismetSystemLibrary|BoxTraceSingleforObjects _returnvalue _returnvalue "200.000000,200.000000,100.000000" "0, 0, 0" (Utilities|Array|MakeArray "ObjectTypeQuery8") false 0 "ForOneFrame" true))
  (Rendering|Material|SetMaterial (Variables|Default|GetBase) 0 (select (or _returnvalue_2 (< (Variables|/Game/FirstPerson/Blueprints/BP_FirstPersonCharacter.BP_FirstPersonCharacter_C|GetMoney (stale EventBeginPlay _returnvalue)) 10)) "/Game/Turret/M_CantBuild.M_CantBuild" "/Game/Turret/M_Build.M_Build"))
  (Variables|Default|SetCanBuild? (not _returnvalue_2)))

(event EventBeginPlay
  (bind _returnvalue (Actor|GetActorOfClass "/Game/FirstPerson/Blueprints/BP_FirstPersonCharacter.BP_FirstPersonCharacter_C")))

(event EventBuildTurret
  (bind _returnvalue (Actor|GetActorOfClass "/Game/FirstPerson/Blueprints/BP_FirstPersonCharacter.BP_FirstPersonCharacter_C"))
  (if (and (Variables|Default|GetCanBuild?) (>= (Variables|/Game/FirstPerson/Blueprints/BP_FirstPersonCharacter.BP_FirstPersonCharacter_C|GetMoney _returnvalue) 15))
    (bind _returnvalue_2 (Actor|GetActorOfClass "/Game/FirstPerson/Blueprints/BP_FirstPersonCharacter.BP_FirstPersonCharacter_C"))
    (Default|SpendMoney _returnvalue_2 15)
    (Game|SpawnActorfromClass (Variables|/Game/FirstPerson/Blueprints/BP_FirstPersonCharacter.BP_FirstPersonCharacter_C|GetTurret _returnvalue_2) (Transformation|GetActorTransform (Variables|/Game/FirstPerson/Blueprints/BP_FirstPersonCharacter.BP_FirstPersonCharacter_C|GetTurret%20Build _returnvalue_2)) "AlwaysSpawn" "MultiplyWithRoot" 0 0)
    (else
      (Development|PrintString "Can't build"))))

(fn ConstructionScript)