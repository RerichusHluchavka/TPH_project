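; Meteor turret Blueprint that drops meteors on guard enemies and can be upgraded by the player.
; Pawn sensing detects a guard and, after a fixed delay, spawns a BP_Meteor above that guard's location.
; A box overlap tracks whether the first-person character is in range.
; The Upgrade event checks range and the player's money, charges the cost, and replaces the turret with BP_MeteorTurretLevel2 at its location.
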(event OnSeePawn(PawnSensing)
  (params (Pawn :type Pawn%20Object%20Reference))
  (bind _asbp_enemy_guard (Utilities|Casting|CastToBP_Enemy_guard Pawn))
  (Utilities|FlowControl|Delay 5.0)
  (Game|SpawnActorfromClass "/Game/Turret/BP_Meteor.BP_Meteor_C" (Math|Transform|MakeTransform (Math|Vector|MakeVector (.x (Transformation|GetActorLocation _asbp_enemy_guard)) (.y (Transformation|GetActorLocation _asbp_enemy_guard)) (+ (.z (Transformation|GetActorLocation _asbp_enemy_guard)) 2e+02)) "0, 0, 0" "1.000000,1.000000,1.000000") "Undefined" "MultiplyWithRoot" self 0))

(event OnComponentBeginOverlap(BoxMeteor)
  (params (OverlappedComponent :type Primitive%20Component%20Object%20Reference) (OtherActor :type Actor%20Object%20Reference) (OtherComp :type Primitive%20Component%20Object%20Reference) (OtherBodyIndex :type Integer) (bFromSweep :type Boolean) (SweepResult :type Hit%20Result%20Structure%20%28by%20ref%29))
  (Utilities|Casting|CastToBP_FirstPersonCharacter OtherActor)
  (Variables|Default|SetInRange? true))

(event OnComponentEndOverlap(BoxMeteor)
  (params (OverlappedComponent :type Primitive%20Component%20Object%20Reference) (OtherActor :type Actor%20Object%20Reference) (OtherComp :type Primitive%20Component%20Object%20Reference) (OtherBodyIndex :type Integer))
  (Utilities|Casting|CastToBP_FirstPersonCharacter OtherActor)
  (Variables|Default|SetInRange? false))

(event EventUpgrade
  (if (Variables|Default|GetInRange?)
    (bind _returnvalue (Actor|GetActorOfClass "/Game/FirstPerson/Blueprints/BP_FirstPersonCharacter.BP_FirstPersonCharacter_C"))
    (if (>= (Variables|/Game/FirstPerson/Blueprints/BP_FirstPersonCharacter.BP_FirstPersonCharacter_C|GetMoney _returnvalue) 30)
      (Default|SpendMoney _returnvalue 30)
      (Actor|DestroyActor)
      (Game|SpawnActorfromClass "/Game/Turret/BP_MeteorTurretLevel2.BP_MeteorTurretLevel2_C" (Math|Transform|MakeTransform (Transformation|GetActorLocation) "0, 0, 0" "1.000000,1.000000,1.000000") "Undefined" "MultiplyWithRoot" 0 0))))

(fn ConstructionScript)

(fn Player
  (return false))