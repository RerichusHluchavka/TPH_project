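; BP_Turret is a level one turret that fires at guard enemies and can be upgraded by the player.
; When PawnSensing sees a BP_Enemy_guard, it waits briefly, then spawns a BP_ProjectileTurret aimed at that guard.
; A box overlap sends a player message and tracks whether something is in range.
; Upgrade, if in range, charges the player character money and replaces the turret with BP_TurretLevel2.
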(event OnSeePawn(PawnSensing)
  (params (Pawn :type Pawn%20Object%20Reference))
  (bind _asbp_enemy_guard (Utilities|Casting|CastToBP_Enemy_guard Pawn))
  (Utilities|FlowControl|Delay 2.0)
  (Game|SpawnActorfromClass "/Game/Turret/BP_ProjectileTurret.BP_ProjectileTurret_C" (Transformation|GetWorldTransform (Variables|Default|GetScene)) "Undefined" "MultiplyWithRoot" self _asbp_enemy_guard 0))

(event OnComponentBeginOverlap(Box)
  (params (OverlappedComponent :type Primitive%20Component%20Object%20Reference) (OtherActor :type Actor%20Object%20Reference) (OtherComp :type Primitive%20Component%20Object%20Reference) (OtherBodyIndex :type Integer) (bFromSweep :type Boolean) (SweepResult :type Hit%20Result%20Structure%20%28by%20ref%29))
  (Class|BPIFirstPersonCharacter|Player(Message) OtherActor)
  (Variables|Default|SetInRange? true))

(event OnComponentEndOverlap(Box)
  (params (OverlappedComponent :type Primitive%20Component%20Object%20Reference) (OtherActor :type Actor%20Object%20Reference) (OtherComp :type Primitive%20Component%20Object%20Reference) (OtherBodyIndex :type Integer))
  (Class|BPIFirstPersonCharacter|Player(Message) OtherActor)
  (Variables|Default|SetInRange? false))

(event EventUpgrade
  (if (Variables|Default|GetInRange?)
    (bind _returnvalue (Actor|GetActorOfClass "/Game/FirstPerson/Blueprints/BP_FirstPersonCharacter.BP_FirstPersonCharacter_C"))
    (if (>= (Variables|/Game/FirstPerson/Blueprints/BP_FirstPersonCharacter.BP_FirstPersonCharacter_C|GetMoney _returnvalue) 20)
      (Default|SpendMoney _returnvalue 20)
      (Actor|DestroyActor)
      (Game|SpawnActorfromClass "/Game/Turret/BP_TurretLevel2.BP_TurretLevel2_C" (Math|Transform|MakeTransform (Transformation|GetActorLocation) "0, 0, 0" "1.000000,1.000000,1.000000") "Undefined" "MultiplyWithRoot" 0 0))))

(fn ConstructionScript)