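; BP_Base is a destructible base that loses health when a BP_Enemy_guard enters its Box trigger.
; Each such overlap calls DecreaseEnemyMessage on the player character, applies damage to the base, spawns BP_Explosion at the enemy and destroys that enemy.
; The value returned by ApplyDamage is subtracted from BaseHealth and the result is printed, with the base destroying itself at zero.
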(event OnComponentBeginOverlap(Box)
  (params (OverlappedComponent :type Primitive%20Component%20Object%20Reference) (OtherActor :type Actor%20Object%20Reference) (OtherComp :type Primitive%20Component%20Object%20Reference) (OtherBodyIndex :type Integer) (bFromSweep :type Boolean) (SweepResult :type Hit%20Result%20Structure%20%28by%20ref%29))
  (bind _asbp_enemy_guard (Utilities|Casting|CastToBP_Enemy_guard OtherActor))
  (Class|BPIDecreaaseEnemy|DecreaseEnemy(Message) (Game|GetPlayerCharacter 0))
  (bind _returnvalue (Game|Damage|ApplyDamage self 1e+01 0 0))
  (Game|SpawnActorfromClass "/Game/Effects/BP_Explosion.BP_Explosion_C" (Math|Conversions|ToTransform(Vector) (Transformation|GetActorLocation _asbp_enemy_guard)) "Undefined" "MultiplyWithRoot" 0 0)
  (Actor|DestroyActor _asbp_enemy_guard)
  (if (> (Variables|Default|GetBase%20Health) 0.0)
    (bind _output_get (Variables|Default|SetBase%20Health (- (Variables|Default|GetBase%20Health) _returnvalue)))
    (Development|PrintString (Utilities|String|ToString(Float) _output_get))
    (if (<= _output_get 0.0)
      (Actor|DestroyActor))))

(fn ConstructionScript)